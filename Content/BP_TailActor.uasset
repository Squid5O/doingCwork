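; BP_TailActor is an actor apparently meant to follow the player, but its logic is unwired, so it does nothing at runtime.
; BeginPlay, Tick and the construction script are empty, though a Korean note states the intent to target the player at spawn.
; Disconnected nodes would store the player pawn as Target and move the actor toward it at Speed, scaled by delta time, without sweep.
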(event EventBeginPlay
  ;[1 1 1] 태어날 때 플레이어를 찾아서 목적지로 하고 싶다.
)

(event Collision|EventActorBeginOverlap
  (params (OtherActor :type Actor%20Object%20Reference)))

(event EventTick
  (params (DeltaSeconds :type Float%20%28single-precision%29))
  ;[1 1 1] 태어날 때 플레이어를 찾아서 목적지로 하고 싶다.
)

(fn ConstructionScript)