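; BP_EnemyActor is an enemy actor Blueprint whose movement logic is disconnected, so BeginPlay, Tick and the construction script do nothing.
; One unwired chain uses a RandomRate roll out of ten to set Direction toward the player pawn or along the actor's forward vector.
; Another unwired chain moves the actor along Direction by Speed and delta time, without sweep.
; Comments show these chains were meant for BeginPlay and Tick.
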(event EventBeginPlay
  ;[1 1 1] 30% 확률로 목적지를 향하는 방향, 나머지 확률로 앞방향.
)

(event Collision|EventActorBeginOverlap
  (params (OtherActor :type Actor%20Object%20Reference)))

(event EventTick
  (params (DeltaSeconds :type Float%20%28single-precision%29))
  ;[1 1 1] 살아가면서 그 방향으로 가고 싶당.
)

(fn ConstructionScript)